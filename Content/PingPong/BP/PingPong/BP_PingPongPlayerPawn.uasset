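; Player pawn for the PingPong game that handles the on-screen score display, with no movement or input logic of its own.
; On BeginPlay it creates WBP_GameScore for player 0, zeroes both scores and adds it to the viewport.
; It then binds to the score-changed dispatcher on each BP_VariablesVault in the level, storing new scores and pushing them to the widget.
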(event `self.ReceiveBeginPlay`
  (`self.CreateWidget`)
  (bind _outactors (`GameplayStatics.GetAllActorsOfClass` "/Game/PingPong/BP/PingPong/BP_VariablesVault.BP_VariablesVault_C"))
  (for _array_element _outactors
    (bind _output_get (set `self.VarVault` _array_element))
    (add `/Game/PingPong/BP/PingPong/BP_VariablesVault.ScoreChanged` _output_get (delegate `ChangeScore`))))

(event `ChangeScore`
  (params (Player1Score :type "Float (double-precision)") (Player2Score :type "Float (double-precision)"))
  (bind _output_get (set `self.Player1Score` Player1Score))
  (bind _output_get_2 (set `self.Player2Score` Player2Score))
  (`self.ChangeWidgetScore` _output_get _output_get_2))

(event `CreateWidget`
  (bind _returnvalue (`|CreateWidget` "/Game/PingPong/UI/WBP_GameScore.WBP_GameScore_C" (`GameplayStatics.GetPlayerController` 0)))
  (bind _output_get (set `self.ScoreWidget` _returnvalue))
  (`/Game/PingPong/UI/WBP_GameScore.ChangeScore` _output_get 0.0 0.0)
  (`UserWidget.AddToViewport` _output_get 0))

(event `ChangeWidgetScore`
  (params (NewParam :type "Float (double-precision)") (NewParam2 :type "Float (double-precision)"))
  (`/Game/PingPong/UI/WBP_GameScore.ChangeScore` (`self.ScoreWidget`) NewParam NewParam2))

(fn `UserConstructionScript`)